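; Speed booster pickup that temporarily or conditionally raises a character's walk speed, built as a child of a pickup parent class.
; It overrides GiveBooster and RemoveBooster, calling the parent first, then setting the character's max walk speed to a hardcoded boosted or normal value.
; Each override also shows or hides the character's speed booster widget.
; The event graph holds no active logic.
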(event EventBeginPlay
  (|CallParentFunction) ; This node is disabled and will not be called.\nDrag off pins to build functionality.
)

(event Collision|EventActorBeginOverlap
  (params (OtherActor :type Actor%20Object%20Reference))
  (|CallParentFunction OtherActor) ; This node is disabled and will not be called.\nDrag off pins to build functionality.
)

(event EventTick
  (params (DeltaSeconds :type Float%20%28single-precision%29))
  (|CallParentFunction DeltaSeconds) ; This node is disabled and will not be called.\nDrag off pins to build functionality.
)

(fn ConstructionScript
  (|CallParentFunction))

(fn GiveBooster
  (params (Character :type BP%20Character%20Base%20Object%20Reference))
  (|CallParentFunction Character)
  (Variables|/Script/Engine.CharacterMovementComponent|SetMaxWalkSpeed (Variables|/Script/Engine.Character|GetCharacterMovement Character) 1.2e+03)
  (Development|SetHiddeninGame (Variables|/Game/ImOnABoatLDJ/Core/Characters/BP_CharacterBase.BP_CharacterBase_C|GetSpeedBoosterWidget Character) false false))

(fn RemoveBooster
  (params (Character :type BP%20Character%20Base%20Object%20Reference))
  (|CallParentFunction Character)
  (Variables|/Script/Engine.CharacterMovementComponent|SetMaxWalkSpeed (Variables|/Script/Engine.Character|GetCharacterMovement Character) 6e+02)
  (Development|SetHiddeninGame (Variables|/Game/ImOnABoatLDJ/Core/Characters/BP_CharacterBase.BP_CharacterBase_C|GetSpeedBoosterWidget Character) true false))