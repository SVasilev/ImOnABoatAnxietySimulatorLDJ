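; BP_PickupBucket is a bucket booster pickup for the boat game that lowers the sinking progress when given to a character.
; GiveBooster runs the parent logic, then cuts the game mode widget's SinkProgressBar percent by a fixed step, writing straight to the UI bar.
; RemoveBooster runs the parent logic, then resets the character's FixSpeed and hides its FixBoosterWidget, though this GiveBooster override sets neither.
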(event EventBeginPlay
  (|CallParentFunction) ; This node is disabled and will not be called.\nDrag off pins to build functionality.
)

(event Collision|EventActorBeginOverlap
  (params (OtherActor :type Actor%20Object%20Reference))
  (|CallParentFunction OtherActor) ; This node is disabled and will not be called.\nDrag off pins to build functionality.
)

(event EventTick
  (params (DeltaSeconds :type Float%20%28single-precision%29))
  (|CallParentFunction DeltaSeconds) ; This node is disabled and will not be called.\nDrag off pins to build functionality.
)

(fn ConstructionScript
  (|CallParentFunction))

(fn GiveBooster
  (params (Character :type BP%20Character%20Base%20Object%20Reference))
  (bind _gamemode (CallFunction|GetImonABoatGameMode))
  (bind _gamewidget (Variables|/Game/ImOnABoatLDJ/Core/GameModes/GM_ImOnABoat.GM_ImOnABoat_C|GetGameWidget _gamemode))
  (bind _sinkprogressbar (Variables|/Game/ImOnABoatLDJ/Core/GameModes/WBP_ImOnABoat.WBP_ImOnABoat_C|GetSinkProgressBar _gamewidget))
  (|CallParentFunction Character)
  (Progress|SetPercent _sinkprogressbar (+ (Variables|/Script/UMG.ProgressBar|GetPercent _sinkprogressbar) -0.1)))

(fn RemoveBooster
  (params (Character :type BP%20Character%20Base%20Object%20Reference))
  (|CallParentFunction Character)
  (Variables|/Game/ImOnABoatLDJ/Core/Characters/BP_CharacterBase.BP_CharacterBase_C|SetFixSpeed Character 1.0)
  (Development|SetHiddeninGame (Variables|/Game/ImOnABoatLDJ/Core/Characters/BP_CharacterBase.BP_CharacterBase_C|GetFixBoosterWidget Character) true false))