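; Base booster pickup that arrives inside a crate and expires 30 seconds after BeginPlay.
; When HitTheGround overlaps a StaticMeshActor, the crate explodes and is destroyed, letting the timeline spin the mesh.
; Once the crate is gone, a character beginning or ending overlap with Box gets the pickup through AcquireBooster, and the actor destroys itself.
; GiveBooster and RemoveBooster are empty here, apparently hooks for child boosters.
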(event OnComponentBeginOverlap(Box)
  (params (OverlappedComponent :type Primitive%20Component%20Object%20Reference) (OtherActor :type Actor%20Object%20Reference) (OtherComp :type Primitive%20Component%20Object%20Reference) (OtherBodyIndex :type Integer) (bFromSweep :type Boolean) (SweepResult :type Hit%20Result%20Structure%20%28by%20ref%29))
  (Utilities|IsValid (Variables|Default|GetCollectibleCrate)
    (:Is%20Not%20Valid
      (bind _asbp_character_base (Utilities|Casting|CastToBP_CharacterBase OtherActor))
      (Default|AcquireBooster _asbp_character_base self)
      (Audio|PlaySound2D "/Game/ImOnABoatLDJ/Art/SFX/InGame/Boost/Activate/MS_BoostActivate_Cue.MS_BoostActivate_Cue" 1.0 1.0 0.0 0 0)
      (Actor|DestroyActor))))

(event OnComponentEndOverlap(Box)
  (params (OverlappedComponent :type Primitive%20Component%20Object%20Reference) (OtherActor :type Actor%20Object%20Reference) (OtherComp :type Primitive%20Component%20Object%20Reference) (OtherBodyIndex :type Integer))
  (Utilities|IsValid (Variables|Default|GetCollectibleCrate)
    (:Is%20Not%20Valid
      (bind _asbp_character_base (Utilities|Casting|CastToBP_CharacterBase OtherActor))
      (Default|AcquireBooster _asbp_character_base self)
      (Audio|PlaySound2D "/Game/ImOnABoatLDJ/Art/SFX/InGame/Boost/Activate/MS_BoostActivate_Cue.MS_BoostActivate_Cue" 1.0 1.0 0.0 0 0)
      (Actor|DestroyActor))))

(event OnComponentBeginOverlap(HitTheGround)
  (params (OverlappedComponent :type Primitive%20Component%20Object%20Reference) (OtherActor :type Actor%20Object%20Reference) (OtherComp :type Primitive%20Component%20Object%20Reference) (OtherBodyIndex :type Integer) (bFromSweep :type Boolean) (SweepResult :type Hit%20Result%20Structure%20%28by%20ref%29))
  (Utilities|Casting|CastToStaticMeshActor OtherActor)
  (Effects|SpawnEmitteratLocation "/Game/StarterContent/Particles/P_Explosion.P_Explosion" (Transformation|GetWorldLocation (Variables|Default|GetCollectibleCrate)) "0, 0, 0" "4.000000,4.000000,4.000000")
  (Components|DestroyComponent (Variables|Default|GetCollectibleCrate))
  (Audio|PlaySound2D "/Game/ImOnABoatLDJ/Art/SFX/InGame/Boost/FallDown/MS_BoostFall_Cue.MS_BoostFall_Cue" 1.0 1.0 0.0 0 0))

(event EventBeginPlay
  (bind _staticmesh (Variables|Default|GetStaticMesh))
  (Actor|SetLifeSpan 3e+01)
  (Audio|PlaySound2D "/Game/ImOnABoatLDJ/Art/SFX/InGame/Boost/FlyIn/MS_BoostFall02_Cue.MS_BoostFall02_Cue" 1.0 1.0 0.0 0 0)
  (bind _rotation (Timeline|Timeline_0 PlayFromStart)
    (:Update
      (Utilities|IsValid (Variables|Default|GetCollectibleCrate)
        (:Is%20Not%20Valid
          (Utilities|IsValid _staticmesh
            (:Is%20Valid
              (Transformation|SetWorldRotation _staticmesh (Math|Rotator|MakeRotator 0.0 0.0 _rotation) false false))))))))

(fn ConstructionScript)

(fn GiveBooster
  (params (Character :type BP%20Character%20Base%20Object%20Reference)))

(fn RemoveBooster
  (params (Character :type BP%20Character%20Base%20Object%20Reference)))