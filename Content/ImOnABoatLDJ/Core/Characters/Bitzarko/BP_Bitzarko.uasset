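; BP_Bitzarko is a character Blueprint that tracks whether the player is throwing at the activity currently in range.
; Each tick it casts CurrentActivityInRange to BP_Throwable and sets IsThrowing while that throwable is active and the first player controller holds Space.
; Throwing pauses the throwable's fly-away timer and releasing unpauses it.
; A debug print of the activity's name is left disconnected.
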(event EventTick
  (params (DeltaSeconds :type Float%20%28single-precision%29))
  (bind _asbp_throwable (Utilities|Casting|CastToBP_Throwable (Variables|Default|GetCurrentActivityInRange))
    (:then
      (bind _output_get (Variables|Default|SetbIsThrowing (and (Variables|/Game/ImOnABoatLDJ/Core/Placeables/BP_ActivityBase.BP_ActivityBase_C|GetbIsActive _asbp_throwable) (Game|Player|IsInputKeyDown (Game|GetPlayerController 0) "SpaceBar"))))
      (if _output_get
        (if (Utilities|Time|IsValidTimerHandle (Variables|/Game/ImOnABoatLDJ/Core/Placeables/BP_Throwable.BP_Throwable_C|GetTimerBeforeFlyAway _asbp_throwable))
          (Utilities|Time|PauseTimerbyHandle (Variables|/Game/ImOnABoatLDJ/Core/Placeables/BP_Throwable.BP_Throwable_C|GetTimerBeforeFlyAway _asbp_throwable)))
        (elif true
          (Utilities|Time|UnpauseTimerbyHandle (Variables|/Game/ImOnABoatLDJ/Core/Placeables/BP_Throwable.BP_Throwable_C|GetTimerBeforeFlyAway _asbp_throwable)))))
    (:CastFailed
      (Variables|Default|SetbIsThrowing false))))

(fn ConstructionScript
  (|CallParentFunction))