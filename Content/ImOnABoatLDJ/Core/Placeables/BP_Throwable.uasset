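; BP_Throwable is a timed crate hazard, worked on via a progress bar, that damages the ship if left active too long.
; Activate shows it and sets timers that speed up WarningBlink, then FlyAway tweens a spawned crate to a random PossibleSlideLocations actor, activates it and explodes.
; DoWork fills the bar on a looping timer and StopWork drains it.
; Deactivate hides it and launches a short-lived physics crate from near BP_Bitzarko.
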(event Custom|IncreaseBar
  (CallFunction|AddtoProgressBar 0.03 true))

(event Custom|StopWork
  (Utilities|Time|ClearandInvalidateTimerbyHandle (Variables|Default|GetGrabbedTimer))
  (CallFunction|AddtoProgressBar -1.0 true))

(event Custom|SpeedUpTheSpline
  (Components|Timeline|SetPlayRate (Variables|Default|GetWarningBlink) 2.0))

(event Custom|FlyAway
  (if (Variables|Default|GetbIsActive)
    (Variables|Default|SetbIsActive false)
    (Rendering|SetActorHiddenInGame true)
    (bind _returnvalue (Game|SpawnActorfromClass "/Script/Engine.StaticMeshActor" (Math|Transform|MakeTransform (Transformation|GetActorLocation) "0, 0, 0" "1,1,1") "Undefined" 0 0))
    (Transformation|SetMobility _returnvalue "Movable")
    (Collision|SetCollisionEnabled (Variables|/Script/Engine.StaticMeshActor|GetStaticMeshComponent _returnvalue) "NoCollision")
    (Components|StaticMesh|SetStaticMesh (Variables|/Script/Engine.StaticMeshActor|GetStaticMeshComponent _returnvalue) "/Game/ImOnABoatLDJ/Art/Gameplay/Throwables/Crate/SM_Crate.SM_Crate")
    (bind _output_get (Variables|Default|SetFixShipToActivate (Utilities|Array|Get(acopy) (Variables|Default|GetPossibleSlideLocations) (Math|Random|RandomIntegerinRange 0 (- (Utilities|Array|Length (Variables|Default|GetPossibleSlideLocations)) 1)))))
    (Variables|Default|SetTargetLocation (- (Transformation|GetActorLocation _output_get) (Transformation|GetActorLocation)))
    (bind _progress (Timeline|Timeline_0 PlayFromStart)
      (:Update
        (Transformation|SetActorLocation _returnvalue (+ (Transformation|GetActorLocation) (* (Variables|Default|GetTargetLocation) _progress)) false true))
      (:Finished
        (Default|Activate (Variables|Default|GetFixShipToActivate))
        (Effects|SpawnEmitteratLocation "/Game/StarterContent/Particles/P_Explosion.P_Explosion" (Transformation|GetActorLocation _returnvalue) "0, 0, 0" "3.000000,3.000000,3.000000")
        (Audio|PlaySound2D "/Game/StarterContent/Audio/Explosion02.Explosion02" 0.1 1.0 0.0 0 0)
        (Actor|DestroyActor _returnvalue)))))

(event Custom|SpeedUpOnceMore
  (Components|Timeline|SetPlayRate (Variables|Default|GetWarningBlink) 5.0))

(event EventDeactivate
  (|CallParentFunction)
  (Rendering|SetActorHiddenInGame true)
  (bind _outactors (Actor|GetAllActorsOfClass "/Game/ImOnABoatLDJ/Core/Characters/Bitzarko/BP_Bitzarko.BP_Bitzarko_C"))
  (bind _returnvalue (Game|SpawnActorfromClass "/Script/Engine.StaticMeshActor" (Math|Transform|MakeTransform (Math|Vector|MakeVector (- (.x (Transformation|GetActorLocation (Utilities|Array|Get(acopy) _outactors))) 1e+02) (.y (Transformation|GetActorLocation (Utilities|Array|Get(acopy) _outactors))) (+ (.z (Transformation|GetActorLocation (Utilities|Array|Get(acopy) _outactors))) 2e+02)) "0, 0, 0" "1,1,1") "Undefined" 0 0))
  (Transformation|SetMobility _returnvalue "Movable")
  (Components|StaticMesh|SetStaticMesh (Variables|/Script/Engine.StaticMeshActor|GetStaticMeshComponent _returnvalue) "/Game/ImOnABoatLDJ/Art/Gameplay/Throwables/Crate/SM_Crate.SM_Crate")
  (Physics|SetSimulatePhysics (Variables|/Script/Engine.StaticMeshActor|GetStaticMeshComponent _returnvalue) true)
  (Physics|AddImpulse (Variables|/Script/Engine.StaticMeshActor|GetStaticMeshComponent _returnvalue) (* (Math|Vector|Normalize (Math|Vector|MakeVector (.x (Math|Vector|RotateVector (Transformation|GetActorForwardVector (Utilities|Array|Get(acopy) _outactors)) "50.000000,180.000000, 0")) (.y (Math|Vector|RotateVector (Transformation|GetActorForwardVector (Utilities|Array|Get(acopy) _outactors)) "50.000000,180.000000, 0")) 0.4)) 2.2e+03) "None" true)
  (Actor|SetLifeSpan _returnvalue 5.0))

(event EventActivate
  (|CallParentFunction)
  (Rendering|SetActorHiddenInGame false)
  (Utilities|Time|SetTimerbyEvent (delegate Custom|SpeedUpTheSpline) (* (Variables|Default|GetSECONDS_BEFORE_FLY) 0.33))
  (Utilities|Time|SetTimerbyEvent (delegate Custom|SpeedUpOnceMore) (* (Variables|Default|GetSECONDS_BEFORE_FLY) 0.66))
  (Utilities|Time|SetTimerbyEvent (delegate Custom|FlyAway) (Variables|Default|GetSECONDS_BEFORE_FLY)))

(event EventDoWork
  (bind _returnvalue (Utilities|Time|SetTimerbyEvent (delegate Custom|IncreaseBar) 0.06 true))
  (Variables|Default|SetGrabbedTimer _returnvalue))

(fn ConstructionScript
  (|CallParentFunction))