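; Base placeable activity that characters can work on, with an IsActive flag toggled by Activate and Deactivate.
; A Box registers it as the overlapping character's CurrentActivityInRange, reasserted every Tick and cleared on exit.
; AddToProgressBar advances a clamped widget bar, optionally resetting and deactivating when full; Tick hides the widget at zero.
; BeginPlay starts a timeline that drives the Warning's opacity through a dynamic material.
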(event OnComponentBeginOverlap(Box)
  (params (OverlappedComponent :type Primitive%20Component%20Object%20Reference) (OtherActor :type Actor%20Object%20Reference) (OtherComp :type Primitive%20Component%20Object%20Reference) (OtherBodyIndex :type Integer) (bFromSweep :type Boolean) (SweepResult :type Hit%20Result%20Structure%20%28by%20ref%29))
  (bind _asbp_character_base (Utilities|Casting|CastToBP_CharacterBase OtherActor))
  (Variables|/Game/ImOnABoatLDJ/Core/Characters/BP_CharacterBase.BP_CharacterBase_C|SetCurrentActivityInRange _asbp_character_base self))

(event OnComponentEndOverlap(Box)
  (params (OverlappedComponent :type Primitive%20Component%20Object%20Reference) (OtherActor :type Actor%20Object%20Reference) (OtherComp :type Primitive%20Component%20Object%20Reference) (OtherBodyIndex :type Integer))
  (bind _asbp_character_base (Utilities|Casting|CastToBP_CharacterBase OtherActor))
  (Variables|/Game/ImOnABoatLDJ/Core/Characters/BP_CharacterBase.BP_CharacterBase_C|SetCurrentActivityInRange _asbp_character_base 0))

(event Custom|Activate
  (Variables|Default|SetbIsActive true))

(event Custom|Deactivate
  (Variables|Default|SetbIsActive false))

(event EventTick
  (params (DeltaSeconds :type Float%20%28single-precision%29))
  (Utilities|FlowControl|Sequence
    (:then_0
      (bind _aswbp_progress_bar (Utilities|Casting|CastToWBP_ProgressBar (UserInterface|GetUserWidgetObject (Variables|Default|GetWidgetComponent))))
      (Development|SetHiddeninGame (Variables|Default|GetWidgetComponent) (<= (Variables|/Script/UMG.ProgressBar|GetPercent (Variables|/Game/ImOnABoatLDJ/Core/Placeables/WBP_ProgressBar.WBP_ProgressBar_C|GetWorkProgressBar _aswbp_progress_bar)) 0.0) false))
    (:then_1
      (for _array_element (Collision|GetOverlappingActors (Variables|Default|GetBox) "/Game/ImOnABoatLDJ/Core/Characters/BP_CharacterBase.BP_CharacterBase_C" :!class /Script/Engine.PrimitiveComponent)
        (bind _asbp_character_base (Utilities|Casting|CastToBP_CharacterBase _array_element))
        (Variables|/Game/ImOnABoatLDJ/Core/Characters/BP_CharacterBase.BP_CharacterBase_C|SetCurrentActivityInRange _asbp_character_base self)))))

(event EventBeginPlay
  (bind _warning (Variables|Default|GetWarning))
  (bind _returnvalue (Rendering|Material|CreateDynamicMaterialInstance _warning 0 (Rendering|Material|GetMaterial _warning 0) "None" :!class /Script/Engine.PrimitiveComponent))
  (Variables|Default|SetNewVar_0 _returnvalue)
  (bind _opacity (Timeline|WarningBlink PlayFromStart)
    (:Update
      (Rendering|Material|SetScalarParameterValue (Variables|Default|GetNewVar_0) "Opacity" _opacity :!class /Script/Engine.MaterialInstanceDynamic))))

(fn ConstructionScript)

(fn AddtoProgressBar
  (params (ValueToAdd :type Float%20%28single-precision%29) (bShouldReset :type Boolean))
  (bind _aswbp_progress_bar (Utilities|Casting|CastToWBP_ProgressBar (UserInterface|GetUserWidgetObject (Variables|Default|GetWidgetComponent))))
  (bind _output_get (LocalVariables|SetNewPercentage (Math|Float|Clamp(Float) (+ (Variables|/Script/UMG.ProgressBar|GetPercent (Variables|/Game/ImOnABoatLDJ/Core/Placeables/WBP_ProgressBar.WBP_ProgressBar_C|GetWorkProgressBar _aswbp_progress_bar)) ValueToAdd))))
  (Default|ChangePercent _aswbp_progress_bar _output_get)
  (if (>= (LocalVariables|GetNewPercentage) 1.0)
    (if bShouldReset
      (Default|ChangePercent _aswbp_progress_bar 0.0)
      (CallFunction|Deactivate))
    (return (LocalVariables|GetNewPercentage))
    (else
      (return (LocalVariables|GetNewPercentage)))))