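; Placeable boat pump hazard that floods when activated, sounding an alarm, showing a puddle and progress bar, and raising the game's sink meter.
; A looping timer fills the local bar and nudges the HUD sink bar while the local one is below full.
; Working it pauses flooding and drains both bars on another timer scaled by BP_Mincho's FixSpeed.
; It deactivates once nearly empty with Mincho in its box, clearing IsPumping.
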(event Custom|IncreaseWaterProgressBar
  (bind _gamemode (CallFunction|GetImonABoatGameMode))
  (bind _gamewidget (Variables|/Game/ImOnABoatLDJ/Core/GameModes/GM_ImOnABoat1.GM_ImOnABoat1_C|GetGameWidget _gamemode))
  (bind _sinkprogressbar (Variables|/Game/ImOnABoatLDJ/Core/GameModes/WBP_ImOnABoat.WBP_ImOnABoat_C|GetSinkProgressBar _gamewidget))
  (bind _currentvalue (CallFunction|AddtoProgressBar 0.1 false))
  (if (< _currentvalue 1.0)
    (Progress|SetPercent _sinkprogressbar (+ (Variables|/Script/UMG.ProgressBar|GetPercent _sinkprogressbar) 0.01))))

(event Custom|StopWork
  (Utilities|Time|UnpauseTimerbyHandle (Variables|Default|GetIncreaseWaterTimer))
  (Utilities|Time|ClearandInvalidateTimerbyHandle (Variables|Default|GetGrabbedTimer)))

(event Custom|RemoveWater
  (bind _gamemode (CallFunction|GetImonABoatGameMode))
  (bind _gamewidget (Variables|/Game/ImOnABoatLDJ/Core/GameModes/GM_ImOnABoat1.GM_ImOnABoat1_C|GetGameWidget _gamemode))
  (bind _sinkprogressbar (Variables|/Game/ImOnABoatLDJ/Core/GameModes/WBP_ImOnABoat.WBP_ImOnABoat_C|GetSinkProgressBar _gamewidget))
  (bind _outactors (Actor|GetAllActorsOfClass "/Game/ImOnABoatLDJ/Core/Characters/Mincho/BP_Mincho.BP_Mincho_C"))
  (bind _currentvalue (CallFunction|AddtoProgressBar (* -0.1 (Variables|/Game/ImOnABoatLDJ/Core/Characters/BP_CharacterBase.BP_CharacterBase_C|GetFixSpeed (Utilities|Array|Get(acopy) _outactors))) true))
  (Progress|SetPercent _sinkprogressbar (Math|Float|Clamp(Float) (+ (Variables|/Script/UMG.ProgressBar|GetPercent _sinkprogressbar) (/ (* -0.1 (Variables|/Game/ImOnABoatLDJ/Core/Characters/BP_CharacterBase.BP_CharacterBase_C|GetFixSpeed (Utilities|Array|Get(acopy) _outactors))) 1e+01))))
  (if (and (> (Utilities|Array|Length (Collision|GetOverlappingActors (Variables|Default|GetBox) "/Game/ImOnABoatLDJ/Core/Characters/Mincho/BP_Mincho.BP_Mincho_C" :!class /Script/Engine.PrimitiveComponent)) 0) (<= _currentvalue 0.01))
    (CallFunction|Deactivate)))

(event Custom|DoWork
  (Utilities|Time|PauseTimerbyHandle (Variables|Default|GetIncreaseWaterTimer))
  (bind _returnvalue (Utilities|Time|SetTimerbyEvent (delegate Custom|RemoveWater) 0.5 true))
  (Variables|Default|SetGrabbedTimer _returnvalue))

(event EventBeginPlay
  (|CallParentFunction)
  (bind _aswbp_progress_bar (Utilities|Casting|CastToWBP_ProgressBar (UserInterface|GetUserWidgetObject (Variables|Default|GetWidgetComponent))))
  (Variables|/Script/UMG.ProgressBar|SetWidgetStyle (Variables|/Game/ImOnABoatLDJ/Core/Placeables/WBP_ProgressBar.WBP_ProgressBar_C|GetWorkProgressBar _aswbp_progress_bar) (Utilities|Struct|MakeProgressBarStyle (Utilities|Struct|MakeSlateBrush "(X=32.000000,Y=32.000000)" "(Left=0.000000,Top=0.000000,Right=0.000000,Bottom=0.000000)" "(SpecifiedColor=(R=1.000000,G=1.000000,B=1.000000,A=1.000000),ColorUseRule=UseColor_Specified)" 0 "NoDrawType" "NoTile" "NoMirror") "(ImageSize=(X=32.000000,Y=32.000000),Margin=(Left=0.000000,Top=0.000000,Right=0.000000,Bottom=0.000000),TintColor=(SpecifiedColor=(R=1.000000,G=1.000000,B=1.000000,A=1.000000),ColorUseRule=UseColor_Specified),ResourceObject=None,ResourceName=\"\",UVRegion=(Min=(X=0.000000,Y=0.000000),Max=(X=0.000000,Y=0.000000),bIsValid=0),DrawAs=Image,Tiling=NoTile,Mirroring=NoMirror,ImageType=NoImage,bIsDynamicallyLoaded=False)" "(ImageSize=(X=32.000000,Y=32.000000),Margin=(Left=0.000000,Top=0.000000,Right=0.000000,Bottom=0.000000),TintColor=(SpecifiedColor=(R=1.000000,G=1.000000,B=1.000000,A=1.000000),ColorUseRule=UseColor_Specified),ResourceObject=None,ResourceName=\"\",UVRegion=(Min=(X=0.000000,Y=0.000000),Max=(X=0.000000,Y=0.000000),bIsValid=0),DrawAs=Image,Tiling=NoTile,Mirroring=NoMirror,ImageType=NoImage,bIsDynamicallyLoaded=False)"))
  (Class|ProgressBar|SetFillColorandOpacity (Variables|/Game/ImOnABoatLDJ/Core/Placeables/WBP_ProgressBar.WBP_ProgressBar_C|GetWorkProgressBar _aswbp_progress_bar) "(R=0.000000,G=0.027330,B=1.000000,A=1.000000)"))

(event Collision|EventActorBeginOverlap
  (params (OtherActor :type Actor%20Object%20Reference))
  (|CallParentFunction OtherActor) ; This node is disabled and will not be called.\nDrag off pins to build functionality.
)

(event EventTick
  (params (DeltaSeconds :type Float%20%28single-precision%29))
  (|CallParentFunction DeltaSeconds))

(event EventActivate
  (|CallParentFunction)
  (Audio|PlaySoundatLocation "/Game/ImOnABoatLDJ/Art/SFX/InGame/Alarm/MS_Alarm.MS_Alarm" (Transformation|GetActorLocation) "0, 0, 0" 1.0 1.0 0.0 0 0 0)
  (Development|SetHiddeninGame (Variables|Default|GetTextRender) false true)
  (Development|SetHiddeninGame (Variables|Default|GetWidgetComponent) false false)
  (Development|SetHiddeninGame (Variables|Default|GetPondMesh) false false)
  (bind _returnvalue (Utilities|Time|SetTimerbyEvent (delegate Custom|IncreaseWaterProgressBar) 1.0 true))
  (Variables|Default|SetIncreaseWaterTimer _returnvalue))

(event EventDeactivate
  (|CallParentFunction)
  (Development|SetHiddeninGame (Variables|Default|GetTextRender) true true)
  (Development|SetHiddeninGame (Variables|Default|GetWidgetComponent) true false)
  (Development|SetHiddeninGame (Variables|Default|GetPondMesh) true false)
  (Utilities|Time|ClearandInvalidateTimerbyHandle (Variables|Default|GetIncreaseWaterTimer))
  (bind _outactors (Actor|GetAllActorsOfClass "/Game/ImOnABoatLDJ/Core/Characters/Mincho/BP_Mincho.BP_Mincho_C"))
  (Variables|/Game/ImOnABoatLDJ/Core/Characters/Mincho/BP_Mincho.BP_Mincho_C|SetbIsPumping (Utilities|Array|Get(acopy) _outactors) false)
  (Utilities|Time|ClearandInvalidateTimerbyHandle (Variables|Default|GetGrabbedTimer)))

(fn ConstructionScript
  (|CallParentFunction))