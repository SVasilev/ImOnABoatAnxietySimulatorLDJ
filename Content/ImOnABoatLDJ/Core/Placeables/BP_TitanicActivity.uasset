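; Timed Titanic-pose event that, once activated, waits up to 20 seconds for two characters to overlap its box.
; Tick triggers a short cinematic: it hides both characters, reveals a stand-in mesh, swaps level audio for flute music and slows time.
; It spawns speed and fix pickups and cuts the sink progress bar by 0.3.
; A timeline pulses the prompt text; the direct ability-boost branch is unwired.
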(event Custom|Timeout
  (Variables|Default|SetbIsActive false)
  (Rendering|SetActorHiddenInGame true))

(event Custom|Activate
  (Rendering|SetActorHiddenInGame false)
  (Variables|Default|SetbIsActive true)
  (Utilities|Time|SetTimerbyEvent (delegate Custom|Timeout) 2e+01))

(event Custom|CustomEvent_1
  ;[1 1 1] Takeaway abilities
  (Utilities|FlowControl|Sequence
    (:then_0
      (bind _outactors (Actor|GetAllActorsOfClass "/Game/ImOnABoatLDJ/Core/Characters/Mincho/BP_Mincho.BP_Mincho_C"))
      (Variables|/Script/Engine.CharacterMovementComponent|SetMaxWalkSpeed (Variables|/Script/Engine.Character|GetCharacterMovement (Utilities|Array|Get(acopy) _outactors)) 6e+02)
      (Development|SetHiddeninGame (Variables|/Game/ImOnABoatLDJ/Core/Characters/BP_CharacterBase.BP_CharacterBase_C|GetSpeedBoosterWidget (Utilities|Array|Get(acopy) _outactors)) true false)
      (Variables|/Game/ImOnABoatLDJ/Core/Characters/BP_CharacterBase.BP_CharacterBase_C|SetFixSpeed (Utilities|Array|Get(acopy) _outactors) 1.0)
      (Development|SetHiddeninGame (Variables|/Game/ImOnABoatLDJ/Core/Characters/BP_CharacterBase.BP_CharacterBase_C|GetFixBoosterWidget (Utilities|Array|Get(acopy) _outactors)) true false))
    (:then_1
      (bind _outactors_2 (Actor|GetAllActorsOfClass "/Game/ImOnABoatLDJ/Core/Characters/Bitzarko/BP_Bitzarko.BP_Bitzarko_C"))
      (Variables|/Script/Engine.CharacterMovementComponent|SetMaxWalkSpeed (Variables|/Script/Engine.Character|GetCharacterMovement (Utilities|Array|Get(acopy) _outactors_2)) 6e+02)
      (Development|SetHiddeninGame (Variables|/Game/ImOnABoatLDJ/Core/Characters/BP_CharacterBase.BP_CharacterBase_C|GetSpeedBoosterWidget (Utilities|Array|Get(acopy) _outactors_2)) true false)
      (Variables|/Game/ImOnABoatLDJ/Core/Characters/BP_CharacterBase.BP_CharacterBase_C|SetFixSpeed (Utilities|Array|Get(acopy) _outactors_2) 1.0)
      (Development|SetHiddeninGame (Variables|/Game/ImOnABoatLDJ/Core/Characters/BP_CharacterBase.BP_CharacterBase_C|GetFixBoosterWidget (Utilities|Array|Get(acopy) _outactors_2)) true false))))

(event EventBeginPlay
  (Variables|Default|SetNewVar_0 "")
  (bind _pulsestrength (Timeline|Pulse PlayFromStart)
    (:Update
      (Transformation|SetWorldScale3D (Variables|Default|GetTextRender) (Math|Vector|MakeVector _pulsestrength _pulsestrength _pulsestrength)))))

(event EventTick
  (params (DeltaSeconds :type Float%20%28single-precision%29))
  (bind _gamemode (CallFunction|GetImonABoatGameMode))
  (bind _box (Variables|Default|GetBox))
  (bind _overlappingactors (Collision|GetOverlappingActors _box "/Game/ImOnABoatLDJ/Core/Characters/BP_CharacterBase.BP_CharacterBase_C" :!class /Script/Engine.PrimitiveComponent))
  (bind _gamewidget (Variables|/Game/ImOnABoatLDJ/Core/GameModes/GM_ImOnABoat1.GM_ImOnABoat1_C|GetGameWidget _gamemode))
  (bind _sinkprogressbar (Variables|/Game/ImOnABoatLDJ/Core/GameModes/WBP_ImOnABoat.WBP_ImOnABoat_C|GetSinkProgressBar _gamewidget))
  (if (Variables|Default|GetbIsActive)
    (if (== (Utilities|Array|Length _overlappingactors) 2)
      (Variables|Default|SetbIsActive false)
      (Utilities|Time|ClearandInvalidateTimerbyHandle (Variables|Default|GetNewVar_0))
      (bind _output_get (Variables|Default|SetOverlapping%20Actors _overlappingactors))
      (for _array_element _output_get
        (Rendering|SetActorHiddenInGame _array_element true))
      (Development|SetHiddeninGame (Variables|Default|GetTextRender) true true)
      (Development|SetHiddeninGame (Variables|Default|GetCylinder2) false true)
      (Audio|Components|Audio|FadeOut (Variables|/Script/Engine.AmbientSound|GetAudioComponent (Variables|Default|GetLevelAudio)) 0.8 0.0 "Linear" :!class /Script/Engine.AudioComponent)
      (Utilities|FlowControl|Delay 1.0)
      (Utilities|Time|SetGlobalTimeDilation 0.2)
      (Audio|PlaySound2D "/Game/ImOnABoatLDJ/Art/SFX/InGame/Titanic/MS_TitanicFlute_Cue.MS_TitanicFlute_Cue" 1.0 1.0 0.0 0 0)
      (Utilities|FlowControl|Sequence
        (:then_0
          (Game|SpawnActorfromClass "/Game/ImOnABoatLDJ/Core/Pickups/BP_Pickup_Speed.BP_Pickup_Speed_C" (Math|Transform|MakeTransform "400.000000,-1780.000000,1500.000000" "0, 0, 0" "1,1,1") "Undefined" 0 0)
          (Game|SpawnActorfromClass "/Game/ImOnABoatLDJ/Core/Pickups/BP_PickupFix.BP_PickupFix_C" (Math|Transform|MakeTransform "440.000000,-1630.000000,1500.000000" "0, 0, 0" "1,1,1") "Undefined" 0 0))
        (:then_1
          (Game|SpawnActorfromClass "/Game/ImOnABoatLDJ/Core/Pickups/BP_Pickup_Speed.BP_Pickup_Speed_C" (Math|Transform|MakeTransform "-400.000000,-1575.000000,1500.000000" "0, 0, 0" "1,1,1") "Undefined" 0 0)
          (Game|SpawnActorfromClass "/Game/ImOnABoatLDJ/Core/Pickups/BP_PickupFix.BP_PickupFix_C" (Math|Transform|MakeTransform "-300.000000,-1740.000000,1500.000000" "0, 0, 0" "1,1,1") "Undefined" 0 0)
          (Utilities|FlowControl|Delay 2.0)
          (Utilities|Time|SetGlobalTimeDilation 1.0)
          (Audio|Components|Audio|FadeIn (Variables|/Script/Engine.AmbientSound|GetAudioComponent (Variables|Default|GetLevelAudio)) 0.8 1.0 (Math|Random|RandomFloatinRange 3e+01 9e+01) "Linear" :!class /Script/Engine.AudioComponent)
          (for _array_element_2 (Variables|Default|GetOverlapping%20Actors)
            (Rendering|SetActorHiddenInGame _array_element_2 false))
          (Rendering|SetActorHiddenInGame true)
          (Development|SetHiddeninGame (Variables|Default|GetCylinder2) true true)
          (Development|SetHiddeninGame (Variables|Default|GetCylinder2) false false)
          (Development|SetHiddeninGame (Variables|Default|GetTextRender) false true)
          (Progress|SetPercent _sinkprogressbar (Math|Float|Clamp(Float) (- (Variables|/Script/UMG.ProgressBar|GetPercent _sinkprogressbar) 0.3))))))))

(fn ConstructionScript)