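; Ship repair placeable that, while active, steadily fills the sink bar on the game mode's widget.
; Activation reveals it, enables collision and teleports the mesh it replaces far below; deactivation reverses this.
; Character work adds to the inherited progress bar, scaled by fix speed, while a looping timer constantly drains it.
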(event Custom|IncreaseSinkBar
  (bind _gamemode (CallFunction|GetImonABoatGameMode))
  (bind _gamewidget (Variables|/Game/ImOnABoatLDJ/Core/GameModes/GM_ImOnABoat1.GM_ImOnABoat1_C|GetGameWidget _gamemode))
  (bind _sinkprogressbar (Variables|/Game/ImOnABoatLDJ/Core/GameModes/WBP_ImOnABoat.WBP_ImOnABoat_C|GetSinkProgressBar _gamewidget))
  (if (Variables|Default|GetbIsActive)
    (Progress|SetPercent _sinkprogressbar (+ (Variables|/Script/UMG.ProgressBar|GetPercent _sinkprogressbar) 0.01))))

(event Custom|DecreaseProgressBar
  (CallFunction|AddtoProgressBar -0.02 true))

(event Custom|DoWork
  (params (Character :type BP%20Character%20Base%20Object%20Reference))
  (CallFunction|AddtoProgressBar (* 0.2 (Variables|/Game/ImOnABoatLDJ/Core/Characters/BP_CharacterBase.BP_CharacterBase_C|GetFixSpeed Character)) true))

(event EventBeginPlay
  (|CallParentFunction)
  (Utilities|Time|SetTimerbyEvent (delegate Custom|IncreaseSinkBar) 1.0 true)
  (Utilities|Time|SetTimerbyEvent (delegate Custom|DecreaseProgressBar) 0.1 true))

(event EventDeactivate
  (|CallParentFunction)
  (Rendering|SetActorHiddenInGame true)
  (Transformation|SetActorLocation (Variables|Default|GetSMToRemove) (Variables|Default|GetInitialLocation) false true)
  (Collision|SetCollisionEnabled (Variables|Default|GetStaticMesh) "NoCollision"))

(event EventActivate
  (bind _smtoremove (Variables|Default|GetSMToRemove))
  (|CallParentFunction)
  (Rendering|SetActorHiddenInGame false)
  (bind _output_get (Variables|Default|SetInitialLocation (Transformation|GetActorLocation _smtoremove)))
  (Transformation|SetActorLocation _smtoremove (- _output_get "0, 0,2000.000000") false true)
  (Collision|SetCollisionEnabled (Variables|Default|GetStaticMesh) "QueryAndPhysics"))

(fn ConstructionScript
  (|CallParentFunction))